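; BP_Enemy is an AI-driven enemy that hunts by sight and sound and ends the game when it spots the player.
; PawnSensing sight of the third-person character shows the lose widget and pauses the game, while any heard noise sends the enemy to that location.
; AIPerception separately moves it to successfully sensed player stimuli and sets an Investigating flag, which this graph never reads.
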(event OnSeePawn(PawnSensing)
  (params (Pawn :type Pawn%20Object%20Reference))
  (Utilities|Casting|CastToBP_ThirdPersonCharacter Pawn)
  (bind _returnvalue (UserInterface|CreateWidget "/Game/Interfaces/YouLooseWidget.YouLooseWidget_C"))
  (UserInterface|Viewport|AddtoViewport _returnvalue 0)
  (Game|SetGamePaused true))

(event OnHearNoise(PawnSensing)
  (params (Instigator :type Pawn%20Object%20Reference) (Location :type Vector%20%28by%20ref%29 :default "0, 0, 0") (Volume :type Float%20%28single-precision%29))
  (AI|AIMoveTo self Location 0 7e+01 false))

(event OnTargetPerceptionUpdated(AIPerception)
  (params (Actor :type Actor%20Object%20Reference) (Stimulus :type AI%20Stimulus%20Structure))
  (bind (_age _expirationage _strength _stimuluslocation _receiverlocation _tag _bsuccessfullysensed) (Utilities|Struct|BreakAIStimulus Stimulus))
  (Utilities|Casting|CastToBP_ThirdPersonCharacter Actor)
  (if _bsuccessfullysensed
    (Variables|Default|SetInvestigating? true)
    (AI|AIMoveTo self _stimuluslocation 0 5.0 false)))

(event EventBeginPlay)

(event Collision|EventActorBeginOverlap
  (params (OtherActor :type Actor%20Object%20Reference)))

(event EventTick
  (params (DeltaSeconds :type Float%20%28single-precision%29)))

(fn ConstructionScript)