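; Game mode that tracks mission objectives and the rock count for a level involving stolen documents and planted bombs.
; BeginPlay resets both objective counters and sets the starting number of rocks.
; Increment functions for documents and bombs each run a completion check, which sets CanFinish once three documents are stolen and one bomb is planted.
; Separate functions raise and lower the rock count without affecting completion.
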(event EventBeginPlay
  (Variables|Default|SetDocsStolen 0)
  (Variables|Default|SetBombsPlanted 0)
  (Variables|Default|SetNumberOfRocks 5))

(fn ConstructionScript)

(fn IncrementBombsPlanted
  (bind _result (Math|Integer|IncrementInt (Variables|Default|GetBombsPlanted))
    (:%20%20
      (Variables|Default|SetBombsPlanted _result)
      (CallFunction|CheckforCompleting))))

(fn IncrementDocsStolen
  (bind _result (Math|Integer|IncrementInt (Variables|Default|GetDocsStolen))
    (:%20%20
      (Variables|Default|SetDocsStolen _result)
      (CallFunction|CheckforCompleting))))

(fn IncrementRocks
  (bind _result (Math|Integer|IncrementInt (Variables|Default|GetNumberOfRocks))
    (:%20%20
      (Variables|Default|SetNumberOfRocks _result))))

(fn DecrementRocks
  (bind _result (Math|Integer|DecrementInt (Variables|Default|GetNumberOfRocks))
    (:%20%20
      (Variables|Default|SetNumberOfRocks _result))))

(fn CheckforCompleting
  (if (and (== (Variables|Default|GetDocsStolen) 3) (== (Variables|Default|GetBombsPlanted) 1))
    (Variables|Default|SetCanFinish true)))