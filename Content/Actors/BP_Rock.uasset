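; BP_Rock is a small throwable rock that makes a distracting noise on impact and can be picked up by the player.
; BeginPlay passes its Velocity variable to ProjectileMovement to launch it.
; Its first Hit, gated by DoOnce, plays a sound and reports a short-range noise event instigated by the player.
; Overlap with BP_ThirdPersonCharacter destroys it and increments the rock count in BP_GameMode.
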(event EventBeginPlay
  (Variables|/Script/Engine.MovementComponent|SetVelocity (Variables|Default|GetProjectileMovement) (Variables|Default|GetVelocity)))

(event Collision|EventActorBeginOverlap
  (params (OtherActor :type Actor%20Object%20Reference))
  (Utilities|Casting|CastToBP_ThirdPersonCharacter OtherActor)
  (Actor|DestroyActor)
  (bind _asbp_game_mode (Utilities|Casting|CastToBP_GameMode (Game|GetGameMode)))
  (Default|IncrementRocks _asbp_game_mode))

(event Collision|EventHit
  (params (MyComp :type Primitive%20Component%20Object%20Reference) (Other :type Actor%20Object%20Reference) (OtherComp :type Primitive%20Component%20Object%20Reference) (bSelfMoved :type Boolean) (HitLocation :type Vector :default "0, 0, 0") (HitNormal :type Vector :default "0, 0, 0") (NormalImpulse :type Vector :default "0, 0, 0") (Hit :type Hit%20Result%20Structure%20%28by%20ref%29))
  (bind _returnvalue (Transformation|GetActorLocation))
  (Utilities|FlowControl|DoOnce false
    (:Completed
      (Audio|PlaySoundatLocation "/Game/Footstep_Tile_Right.Footstep_Tile_Right" _returnvalue "0, 0, 0" 1.0 1.0 0.0 0 0 0 0)
      (Class|AISenseHearing|ReportNoiseEvent _returnvalue 1.0 (Game|GetPlayerCharacter 0) 5e+02 "None"))))

(fn ConstructionScript
  (Transformation|SetWorldScale3D (Variables|Default|GetStaticMesh) "0.250000,0.250000,0.250000"))