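; BP_Bomb is a plant site where the player interacts to place a bomb.
; Overlap with its Box shows an interact widget to BP_ThirdPersonCharacter and removes it on exit.
; The first Interact call removes the prompt, destroys the Plane and Box components, reveals the Bomb and increments the planted count in BP_GameMode.
; A ButtonPressed flag makes planting one-shot.
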(event OnComponentBeginOverlap(Box)
  (params (OverlappedComponent :type Primitive%20Component%20Object%20Reference) (OtherActor :type Actor%20Object%20Reference) (OtherComp :type Primitive%20Component%20Object%20Reference) (OtherBodyIndex :type Integer) (bFromSweep :type Boolean) (SweepResult :type Hit%20Result%20Structure%20%28by%20ref%29))
  (if (not (Variables|Default|GetButtonPressed))
    (Utilities|Casting|CastToBP_ThirdPersonCharacter OtherActor)
    (bind _returnvalue (UserInterface|CreateWidget "/Game/Interfaces/Interact_WIdget.Interact_WIdget_C"))
    (UserInterface|Viewport|AddtoViewport _returnvalue 0)))

(event OnComponentEndOverlap(Box)
  (params (OverlappedComponent :type Primitive%20Component%20Object%20Reference) (OtherActor :type Actor%20Object%20Reference) (OtherComp :type Primitive%20Component%20Object%20Reference) (OtherBodyIndex :type Integer))
  (Utilities|Casting|CastToBP_ThirdPersonCharacter OtherActor)
  (Widget|RemovefromParent (stale OnComponentBeginOverlap(Box) _returnvalue)))

(event EventInteract
  (if (not (Variables|Default|GetButtonPressed))
    (Variables|Default|SetButtonPressed true)
    (Widget|RemovefromParent (stale OnComponentBeginOverlap(Box) _returnvalue))
    (Components|DestroyComponent (Variables|Default|GetPlane))
    (Components|DestroyComponent (Variables|Default|GetBox))
    (Rendering|SetVisibility (Variables|Default|GetBomb) true false)
    (bind _asbp_game_mode (Utilities|Casting|CastToBP_GameMode (Game|GetGameMode)))
    (bind _output_get (Variables|Default|SetGameMode _asbp_game_mode))
    (Default|IncrementBombsPlanted _output_get)))

(fn ConstructionScript)